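; Base ability component for the FPS character that provides shared activation, stamina cost and cooldown handling for child abilities.
; On BeginPlay it caches the owner's stamina and gameplay tag components and loads its data from DT_AbilityData by AbilityName.
; Activation checks stamina, cooldown and tag, then starts the timer, runs overridable AbilityLogic, adds the tag and spends stamina.
; EndAbility removes the tag, while CancelAbility and PopulateAbilityData are empty stubs.
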(event `self.ReceiveBeginPlay`
  (`|ExecutionSequence`
    (:`then_0`
      (bind _asbp_fpscharacter (cast `/Game/Player/Character/BP_FPSCharacter` (`self.GetOwner`)))
      (set `self.FPSCharacter` _asbp_fpscharacter)
      (set `self.Comp_Stamina` (`Actor.GetComponentByClass` (`self.GetOwner`) "/Game/Components/Comp_Stamina.Comp_Stamina_C"))
      (set `self.Comp_GameplayTags` (`Actor.GetComponentByClass` (`self.GetOwner`) "/Game/Components/Comp_GameplayTags.Comp_GameplayTags_C")))
    (:`then_1`
      (bind _returnvalue (`|GetDataTableRow` "/Game/DataTables/DT_AbilityData.DT_AbilityData" (`self.AbilityName`))
        (:`then`
          (set `self.AbilityData` _returnvalue))))))

(fn `AbilityLogic`
  (params (TargetActor :type "Actor Object Reference"))
  (`KismetSystemLibrary.PrintString` "No Ability Logic Added (Remove Parent to remove this message)"))

(fn `ActivateAbility`
  (params (TargetActor :type "Actor Object Reference"))
  (if (`self.CanActivateAbility?`)
    (`self.StartAbilityCooldown`)
    (`self.AbilityLogic` TargetActor)
    (`/Game/Components/Comp_GameplayTags.AddGameplayTag` (`self.Comp_GameplayTags`) (`.GameplayTag_15_063864724033F9373D31C39F9A61D8B7` (break `/Game/Structs/S_AbilityData` (`self.AbilityData`))))
    (`self.HandleAbilityCost`)))

(fn `CanActivateAbility?`
  (returns (`CanActivate?` :type Boolean))
  (bind ((`AbilityClass_18_F2DCBAB4451FD8A20279148CEC54BCBE` _abilityclass) (`Cost_7_EB16A90D4F20CD0243D73F9496C8B2C6` _cost) (`GameplayTag_15_063864724033F9373D31C39F9A61D8B7` _gameplaytag)) (break `/Game/Structs/S_AbilityData` (`self.AbilityData`)))
  (return (and (`/Game/Components/Comp_Stamina.HasStamina?` (`self.Comp_Stamina`) _cost) (not (`self.InCooldown?`)) (not (`/Game/Components/Comp_GameplayTags.HasTag` (`self.Comp_GameplayTags`) _gameplaytag false)))))

(fn `CancelAbility`)

(fn `EndAbility`
  (`/Game/Components/Comp_GameplayTags.RemoveGameplayTag` (`self.Comp_GameplayTags`) (`.GameplayTag_15_063864724033F9373D31C39F9A61D8B7` (break `/Game/Structs/S_AbilityData` (`self.AbilityData`)))))

(fn `EndAbilityCooldown`
  (set `self.InCooldown?` false))

(fn `HandleAbilityCost`
  (`/Game/Components/Comp_Stamina.DecreaseStamina` (`self.Comp_Stamina`) (`.Cost_7_EB16A90D4F20CD0243D73F9496C8B2C6` (break `/Game/Structs/S_AbilityData` (`self.AbilityData`))))
  (`/Game/Components/Comp_Stamina.RecoverStaminaLoopStart` (`self.Comp_Stamina`)))

(fn `PopulateAbilityData`)

(fn `StartAbilityCooldown`
  (`KismetSystemLibrary.K2_SetTimer` null "EndAbilityCooldown" (`.Cooldown_5_4339A1634C3C00DE7FC834AC7D777B83` (break `/Game/Structs/S_AbilityData` (`self.AbilityData`))))
  (set `self.InCooldown?` true))