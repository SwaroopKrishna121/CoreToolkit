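; Dash ability component that gives the FPS character a short burst of speed when its ability logic runs.
; StartDash saves velocity and ground friction, zeroes friction, and sets velocity to a calculated vector times DashForce.
; A short timer calls EndDash, which restores both saved values.
; CalculateLocationAfterDash holds a last-input-or-forward direction selection, though that node appears unconnected.
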(fn `AbilityLogic`
  (params (TargetActor :type "Actor Object Reference"))
  (`self.StartDash`))

(fn `EndDash`
  (set `CharacterMovementComponent.GroundFriction` (`self.DefaultGroundFriction`) (`Character.CharacterMovement` (`self.FPSCharacter`)))
  (set `MovementComponent.Velocity` (`self.DefaultVelocity`) (`Character.CharacterMovement` (`self.FPSCharacter`))))

(fn `StartDash`
  (set `self.DefaultVelocity` (`MovementComponent.Velocity` (`Character.CharacterMovement` (`self.FPSCharacter`))))
  (set `self.DefaultGroundFriction` (`CharacterMovementComponent.GroundFriction` (`Character.CharacterMovement` (`self.FPSCharacter`))))
  (set `CharacterMovementComponent.GroundFriction` 0.0 (`Character.CharacterMovement` (`self.FPSCharacter`)))
  (set `MovementComponent.Velocity` (* (`self.CalculateLocationAfterDash`) (`self.DashForce`)) (`Character.CharacterMovement` (`self.FPSCharacter`)))
  (`KismetSystemLibrary.K2_SetTimer` null "EndDash" 0.2))