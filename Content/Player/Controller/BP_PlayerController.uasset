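; BP_PlayerController is the first-person player's controller, setting up input and the HUD at the start of play.
; On BeginPlay it caches the BP_FPSCharacter, adds the IMC_Default Enhanced Input mapping context, then creates WBP_HUD and adds it to the viewport.
; Each Tick it polls whether the character's InteractableActor is valid and passes that to the HUD to update the crosshair icon.
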(event `self.ReceiveBeginPlay`
  (bind _asbp_fpscharacter (cast `/Game/Player/Character/BP_FPSCharacter` (`GameplayStatics.GetPlayerCharacter` 0)))
  (bind _output_get (set `self.FPSCharacter` _asbp_fpscharacter))
  (`/Engine/EditorBlueprintResources/StandardMacros.IsValid` _output_get
    (:`Is Valid`
      (`|ExecutionSequence`
        (:`then_0`
          (`EnhancedInputSubsystemInterface.AddMappingContext` (pcsubsystem `EnhancedInputLocalPlayerSubsystem` self) "/Game/Player/Input/IMC_Default.IMC_Default" 0 (struct)))
        (:`then_1`
          (bind _returnvalue (`|CreateWidget` "/Game/UI/WBP_HUD.WBP_HUD_C" self))
          (bind _output_get_2 (set `self.HUD` _returnvalue))
          (`UserWidget.AddToViewport` _output_get_2 0))))))

(event `self.ReceiveTick`
  (params (DeltaSeconds :type "Float (single-precision)"))
  (`self.UpdateCrosshairIcon`))

(fn `UpdateCrosshairIcon`
  (`/Game/UI/WBP_HUD.UpdateCrosshairIcon` (`self.HUD`) (`KismetSystemLibrary.IsValid` (`/Game/Player/Character/BP_FPSCharacter.InteractableActor` (`self.FPSCharacter`)))))

(fn `UserConstructionScript`)