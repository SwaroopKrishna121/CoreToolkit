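; Trigger volume that blocks a configurable list of abilities for actors tagged AbilityActor while they overlap it.
; On begin overlap, it removes each listed ability the actor has through its Comp_AbilitySystem component.
; On end overlap, it adds every listed ability the actor lacks, without tracking whether the actor had it on entry.
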(event `self.Trigger.OnComponentBeginOverlap`
  (params (OverlappedComponent :type "PrimitiveComponent Object Reference") (OtherActor :type "Actor Object Reference") (OtherComp :type "PrimitiveComponent Object Reference") (OtherBodyIndex :type Integer) (bFromSweep :type Boolean) (SweepResult :type "HitResult Structure (by ref)"))
  (bind _returnvalue (`self.GetComponentByClass` OtherActor "/Game/Components/Comp_AbilitySystem.Comp_AbilitySystem_C"))
  (if (`self.ActorHasTag` OtherActor "AbilityActor")
    (for _array_element (`self.AbilitiesToBlock`)
      (if (`/Game/Components/Comp_AbilitySystem.HasAbility` _returnvalue _array_element)
        (`/Game/Components/Comp_AbilitySystem.RemoveAbility` _returnvalue _array_element)))))

(event `self.Trigger.OnComponentEndOverlap`
  (params (OverlappedComponent :type "PrimitiveComponent Object Reference") (OtherActor :type "Actor Object Reference") (OtherComp :type "PrimitiveComponent Object Reference") (OtherBodyIndex :type Integer))
  (bind _returnvalue (`self.GetComponentByClass` OtherActor "/Game/Components/Comp_AbilitySystem.Comp_AbilitySystem_C"))
  (if (`self.ActorHasTag` OtherActor "AbilityActor")
    (for _array_element (`self.AbilitiesToBlock`)
      (if (not (`/Game/Components/Comp_AbilitySystem.HasAbility` _returnvalue _array_element))
        (`/Game/Components/Comp_AbilitySystem.AddAbility` _returnvalue _array_element)))))

(fn `UserConstructionScript`)